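; Lock actor that a RoguePawn picks by staying inside its overlap for PickTime seconds.
; While picking, Tick drains LockHealth and lerps a dynamic material's Color from its starting value toward red as progress feedback.
; Leaving early resets both timer and color.
; When health runs out, the lock is marked picked, its Cube and Sphere start simulating physics, and the actor expires after a short lifespan.
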(event EventBeginPlay
  (bind _returnvalue (Rendering|Material|CreateDynamicMaterialInstance (Variables|Default|GetCube) 0 "/Game/Materials/TempLockMaterial.TempLockMaterial" "None" :!class /Script/Engine.PrimitiveComponent))
  (bind _output_get (Variables|Default|SetDynamicMaterial _returnvalue))
  (Rendering|Material|SetMaterial (Variables|Default|GetCube) 0 _output_get)
  (bind _returnvalue_2 (Rendering|Material|GetVectorParameterValue (Variables|Default|GetDynamicMaterial) "Color" :!class /Script/Engine.MaterialInstanceDynamic))
  (Variables|Default|SetStartingColor _returnvalue_2)
  (Variables|Default|SetLockHealth (Variables|Default|GetPickTime)))

(event Collision|EventActorBeginOverlap
  (params (OtherActor :type Actor%20Object%20Reference))
  (Utilities|Casting|CastToRoguePawn OtherActor)
  (Variables|Default|SetPicking true))

(event EventTick
  (params (DeltaSeconds :type Float%20%28single-precision%29))
  (if (and (Variables|Default|GetPicking) (not (Variables|Default|GetPicked)))
    (Variables|Default|SetLockHealth (- (Variables|Default|GetLockHealth) (* DeltaSeconds 1.0)))
    (Rendering|Material|SetVectorParameterValue (Variables|Default|GetDynamicMaterial) "Color" (Math|Color|Lerp(LinearColor) "(R=0.604167,G=0.010489,B=0.000000,A=1.000000)" (Variables|Default|GetStartingColor) (/ (Variables|Default|GetLockHealth) (Variables|Default|GetPickTime))) :!class /Script/Engine.MaterialInstanceDynamic)
    (if (<= (Variables|Default|GetLockHealth) 0.0)
      (Variables|Default|SetPicked true)
      (Physics|SetSimulatePhysics (Variables|Default|GetSphere) true)
      (Physics|SetSimulatePhysics (Variables|Default|GetCube) true)
      (Actor|SetLifeSpan 5.0))))

(event Collision|EventActorEndOverlap
  (params (OtherActor :type Actor%20Object%20Reference))
  (Utilities|Casting|CastToRoguePawn OtherActor)
  (Variables|Default|SetPicking false)
  (if (> (Variables|Default|GetLockHealth) 0.0)
    (Variables|Default|SetLockHealth (Variables|Default|GetPickTime))
    (Rendering|Material|SetVectorParameterValue (Variables|Default|GetDynamicMaterial) "Color" (Variables|Default|GetStartingColor) :!class /Script/Engine.MaterialInstanceDynamic)))

(fn ConstructionScript)
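; LoreBook1 is an interactable lore book actor that opens a reading widget when the player interacts with it.
; Hover and UnHover events show and hide its interaction prompt widget.
; Interact adds LoreBook1Widget to the viewport, shows the mouse cursor, destroys the book and switches input to UI-only.
; Logic to turn the prompt toward the player around the vertical axis exists but is disconnected and never runs.
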(event EventHover
  ;[0 1 0.9817] Interact & Hover Events - David Wills
  (Rendering|SetVisibility (Variables|Default|GetWidget) true false))

(event EventUnHover
  ;[0 1 0.9817] Interact & Hover Events - David Wills
  (Rendering|SetVisibility (Variables|Default|GetWidget) false false))

(event EventInteract
  (bind _returnvalue (Game|GetPlayerController 0))
  ;[0 1 0.9817] Interact & Hover Events - David Wills
  (bind _returnvalue_2 (UserInterface|CreateWidget "/Game/Widget/LoreBooks/LoreBook1Widget.LoreBook1Widget_C"))
  (UserInterface|Viewport|AddtoViewport _returnvalue_2 0)
  (Variables|/Script/Engine.PlayerController|SetbShowMouseCursor _returnvalue true)
  (Actor|DestroyActor)
  (Input|SetInputModeUIOnly _returnvalue _returnvalue_2 "DoNotLock"))

(fn ConstructionScript)
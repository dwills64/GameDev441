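; NextLevel is a level-exit trigger that opens the next numbered level when any Pawn overlaps it.
; On BeginPlay it increments the last character of the current level name, builds a "Level" plus number name from it, and prints that name.
; Only the final digit is read, so numbering past single digits is not handled.
; Tick spins the Capsule around yaw at a constant, frame-rate independent speed.
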(event EventBeginPlay
  (bind _returnvalue (Game|GetCurrentLevelName true))
  (bind _output_get (Variables|Default|SetnextLevel (Utilities|String|Right _returnvalue 1)))
  (bind _result (Math|Integer|IncrementInt (Math|Conversions|ToInteger(Byte) _output_get))
    (:%20%20
      (bind _output_get_2 (Variables|Default|SetnextLevelName (Utilities|String|StringToName (Utilities|String|Append "Level" (Utilities|String|ToString(Integer) _result)))))
      (Development|PrintString (Utilities|String|ToString(Name) _output_get_2)))))

(event Collision|EventActorBeginOverlap
  (params (OtherActor :type Actor%20Object%20Reference))
  (Utilities|Casting|CastToPawn OtherActor)
  (Game|OpenLevel(byName) (Variables|Default|GetnextLevelName)))

(event EventTick
  (params (DeltaSeconds :type Float%20%28single-precision%29))
  (Transformation|AddLocalRotation (Variables|Default|GetCapsule) (Math|Rotator|MakeRotator 0.0 0.0 (* DeltaSeconds 6e+01)) false false))

(fn ConstructionScript)

(fn NewFunction0)
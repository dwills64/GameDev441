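; Birb is a bird NPC that scavenges around its spawn point until the player comes near, then flies away.
; Each Tick, Scavenge checks squared player distance and picks random reachable navmesh points on arrival, using a random timer to gate the next pick.
; Once spooked, it takes the player's rotation, climbs forward by local offsets and destroys itself above an exit height.
; CheckForThreat is an uncalled variant of CheckSpook.
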(event EventBeginPlay
  ;[1 1 1] Birb NPC by Dylan Sturgeon, heavily based off provided in-class examples (thank you!)
  (bind _output_get (Variables|Default|SetStartingPoint (Transformation|GetActorLocation)))
  (bind _output_get_2 (Variables|Default|SetNextPoint _output_get))
  (Variables|Default|SetExitHeight (+ (.z _output_get_2) (Variables|Default|GetExitHeight))))

(event Collision|EventActorBeginOverlap
  (params (OtherActor :type Actor%20Object%20Reference))
  ;[1 1 1] Birb NPC by Dylan Sturgeon, heavily based off provided in-class examples (thank you!)
)

(event EventTick
  (params (DeltaSeconds :type Float%20%28single-precision%29))
  (bind _flightspeed (Variables|Default|GetFlightSpeed))
  ;[1 1 1] Birb NPC by Dylan Sturgeon, heavily based off provided in-class examples (thank you!)
  (if (Variables|Default|GetSpooked)
    (Transformation|AddActorLocalOffset (Math|Vector|MakeVector (* _flightspeed DeltaSeconds) 0.0 (* _flightspeed DeltaSeconds)) false false)
    (if (> (.z (Transformation|GetActorLocation)) (Variables|Default|GetExitHeight))
      (Actor|DestroyActor))
    (else
      (CallFunction|Scavenge))))

(fn ConstructionScript)

(fn CheckforThreat
  (bind _returnvalue (Game|Player|GetPlayerPawn 0))
  (bind _returnvalue_2 (Transformation|GetActorRotation _returnvalue))
  (if (<= (Class|KismetMathLibrary|VectorDistanceSquared (Transformation|GetActorLocation (Game|Player|GetPlayerPawn 0)) (Transformation|GetActorLocation)) (Variables|Default|GetSpookRange))
    (Variables|Default|SetSpooked true)
    (Transformation|SetActorRotation (Math|Rotator|MakeRotator 0.0 (.pitch _returnvalue_2) (.yaw _returnvalue_2)))
    (else
      (Variables|Default|SetSpooked false)
      (Utilities|Time|SetTimerbyFunctionName 0 "CheckForIThreat" 0.0))))

(fn Scavenge
  (CallFunction|CheckSpook)
  ;[1 1 1] Don't wander again until Timer is up.
  (if (not (Variables|Default|GetSpooked))
    (if (Variables|Default|GetMove)
      ;[1 1 1] Check if we have reached our wander point.
      (if (<= (Math|Vector|Distance(Vector) (Transformation|GetActorLocation) (Variables|Default|GetNextPoint)) 1.5e+02)
        ;[1 1 1] If we've reached our target, stop for a time.
        (Variables|Default|SetMove false)
        (Utilities|Time|SetTimerbyFunctionName 0 "MovePermission" (Math|Random|RandomFloatinRange 1.0 3.0))
        (Variables|Default|SetNextPoint (.RandomLocation (AI|Navigation|GetRandomReachablePointinRadius (Variables|Default|GetStartingPoint) (Variables|Default|GetScavengeRange) 0 0)))
        (AI|Navigation|SimpleMovetoLocation (Pawn|GetController) (Variables|Default|GetNextPoint))))))

(fn MovePermission
  (Variables|Default|SetMove true))

(fn CheckSpook
  (if (<= (Class|KismetMathLibrary|VectorDistanceSquared (Transformation|GetActorLocation (Game|Player|GetPlayerPawn 0)) (Transformation|GetActorLocation)) (Math|Float|Square (Variables|Default|GetSpookRange)))
    (Variables|Default|SetSpooked true)
    (Transformation|SetWorldRotation (Variables|Default|GetDefaultSceneRoot) (Transformation|GetActorRotation (Game|Player|GetPlayerPawn 0)) false false)
    (else
      (return))))
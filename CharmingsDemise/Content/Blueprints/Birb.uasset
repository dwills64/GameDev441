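; Birb is a bird pawn that wanders around its starting point and can be spooked by the player.
; CheckForThreat turns it to the player's facing when within SpookRange, otherwise sets a timer for misspelled "CheckForIThreat".
; Scavenge, gated by Move, picks and walks to a random reachable point on arrival, clearing CanWander and timing MovePermission to set Move.
; Event graph stubs are empty, so nothing here starts either behavior.
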(event EventBeginPlay)

(event Collision|EventActorBeginOverlap
  (params (OtherActor :type Actor%20Object%20Reference)))

(event EventTick
  (params (DeltaSeconds :type Float%20%28single-precision%29)))

(fn ConstructionScript)

(fn CheckforThreat
  (bind _returnvalue (Game|Player|GetPlayerPawn 0))
  (bind _returnvalue_2 (Transformation|GetActorRotation _returnvalue))
  (if (<= (Class|KismetMathLibrary|VectorDistanceSquared (Transformation|GetActorLocation (Game|Player|GetPlayerPawn 0)) (Transformation|GetActorLocation)) (Variables|Default|GetSpookRange))
    (Variables|Default|SetSpooked true)
    (Transformation|SetActorRotation (Math|Rotator|MakeRotator 0.0 (.pitch _returnvalue_2) (.yaw _returnvalue_2)))
    (else
      (Variables|Default|SetSpooked false)
      (Utilities|Time|SetTimerbyFunctionName 0 "CheckForIThreat" (Variables|Default|GetAttentionSpan)))))

(fn Scavenge
  ;[1 1 1] Don't wander again until Timer is up.
  (if (Variables|Default|GetMove)
    ;[1 1 1] Check if we have reached our wander point.
    (if (<= (Math|Vector|Distance(Vector) (Transformation|GetActorLocation) (Variables|Default|GetNextPoint)) 1.5e+02)
      ;[1 1 1] If we've reached our target, stop for a time.
      (Variables|Default|SetCanWander false)
      (Utilities|Time|SetTimerbyFunctionName 0 "MovePermission" (Math|Random|RandomFloatinRange 1.0 3.0))
      (Variables|Default|SetNextPoint (.RandomLocation (AI|Navigation|GetRandomReachablePointinRadius (Variables|Default|GetStartingPoint) (Variables|Default|GetRadius) 0 0)))
      (AI|Navigation|SimpleMovetoLocation (Pawn|GetController) (Variables|Default|GetNextPoint)))))

(fn MovePermission
  (Variables|Default|SetMove true))